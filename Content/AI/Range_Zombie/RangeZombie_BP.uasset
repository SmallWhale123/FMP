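; RangeZombie_BP is a zombie enemy that reports health and player sighting or damage to its AI blackboard.
; AttackPlayer sphere-traces forward, then plays a random attack montage, or moves in to bite a nearby dead player.
; Left and right hand socket traces deal damage, or drain stamina from a blocking player, using a HitPlayer guard.
; Lethal damage stops the AI, raises player favour, plays death effects and destroys the actor.
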(event OnSeePawn(PawnSensing)
  (params (Pawn :type Pawn%20Object%20Reference))
  ;[1 1 1] Sensing Player
  (Utilities|Casting|CastToBP_ThirdPersonCharacter Pawn)
  (AI|Components|Blackboard|SetValueasBool (AI|GetBlackboard (AI|GetAIController self)) (Utilities|Name|MakeLiteralName "HasSeenPlayer?") true))

(event Custom|Die
  ;[1 1 1] Death
  (Variables|Default|SetDead true)
  (bind _asweak_zombie_controller (Utilities|Casting|CastToWeak_ZombieController (Pawn|GetController)))
  (Default|StopAI _asweak_zombie_controller)
  (Pawn|Components|CharacterMovement|DisableMovement (Variables|Character|GetCharacterMovement))
  (bind _asbp_third_person_character (Utilities|Casting|CastToBP_ThirdPersonCharacter (Game|GetPlayerCharacter 0)))
  (Default|IncreaseFavour _asbp_third_person_character 5.0)
  (Components|Animation|PlayAnimation (Variables|Character|GetMesh) (Utilities|Select :Index (Math|Random|RandomIntegerinRange 0 1) :Option%200 "/Game/AI/Weak_Zombie/Animation/Combat/Zombie_Dying_Montage.Zombie_Dying_Montage" :Option%201 "/Game/AI/Weak_Zombie/Animation/Combat/Zombie_Death_Montage.Zombie_Death_Montage") false)
  (Audio|PlaySoundatLocation (Utilities|Select :Index (Math|Random|RandomIntegerinRange 0 1) :Option%200 "/Game/Audio/ZombieGroans/ZombieDeath1.ZombieDeath1" :Option%201 "/Game/Audio/ZombieGroans/ZombieDeath2.ZombieDeath2") (Transformation|GetWorldLocation (Variables|Character|GetMesh)) "0, 0, 0" 1.0 1.0 0.0 0 0 0 0)
  (Utilities|FlowControl|Delay 5.0)
  (Actor|DestroyActor))

(event Custom|AttackPlayer
  (bind _returnvalue (Transformation|GetActorLocation))
  ;[1 1 1] Attack Player/Player Death Interaction
  (bind _returnvalue_2 (Actor|GetActorOfClass "RangeZombie_BP_C"))
  (bind (_outhit _returnvalue_3) (Collision|SphereTraceForObjects _returnvalue (+ _returnvalue (* (Math|Vector|GetForwardVector (Transformation|GetActorRotation)) 3e+02)) 1.2e+02 (Utilities|Array|MakeArray "ObjectTypeQuery3") false (Utilities|Array|MakeArray _returnvalue_2) "None"))
  (if _returnvalue_3
    ;[1 1 1] player Death Interraction
    (bind _asbp_third_person_character (Utilities|Casting|CastToBP_ThirdPersonCharacter (.HitActor (Collision|BreakHitResult _outhit))))
    (if (<= (Variables|/Game/ThirdPerson/Blueprints/BP_ThirdPersonCharacter.BP_ThirdPersonCharacter_C|GetCurrentHealth _asbp_third_person_character) 0.0)
      (if (<= (.Distance (Collision|BreakHitResult _outhit)) 4e+01)
        (AI|AIMoveTo (AI|GetAIController self) (Transformation|GetWorldLocation (Variables|/Script/Engine.Character|GetMesh _asbp_third_person_character)) 0 -1.0 "Default" "Default" true false
          (:then
            (Components|Animation|PlayAnimation (Variables|Character|GetMesh) "/Game/AI/Weak_Zombie/Animation/Combat/Zombie_Biting_Montage.Zombie_Biting_Montage" true))))
      (else
        ;[1 1 1] Attack Player Normally
        (Animation|Montage|PlayMontage (Variables|Character|GetMesh) (Utilities|Select :Index (Math|Random|RandomIntegerinRange 0 1) :Option%200 "/Game/AI/Weak_Zombie/Animation/Combat/Zombie_Attack_Montage.Zombie_Attack_Montage" :Option%201 "/Game/AI/Weak_Zombie/Animation/Combat/Zombie_Attack__1__Montage.Zombie_Attack__1__Montage")
          (:OnCompleted
            _)
          (:OnInterrupted
            _))
        (Variables|Default|SetHitPlayer false)
        (Audio|PlaySoundatLocation (Utilities|Select :Index (Math|Random|RandomIntegerinRange 0 1) :Option%200 "/Game/Audio/ZombieGroans/ZombieAttack1.ZombieAttack1" :Option%201 "/Game/Audio/ZombieGroans/ZombieAttack2.ZombieAttack2") (Transformation|GetWorldLocation (Variables|Character|GetMesh)) "0, 0, 0" 1.0 1.0 0.0 0 0 0 0)))))

(event Game|Damage|EventAnyDamage
  (params (Damage :type Float%20%28single-precision%29) (DamageType :type Damage%20Type%20Object%20Reference) (InstigatedBy :type Controller%20Object%20Reference) (DamageCauser :type Actor%20Object%20Reference))
  ;[1 1 1] Taking Damage
  (AI|Components|Blackboard|SetValueasBool (AI|GetBlackboard (AI|GetAIController self)) (Utilities|Name|MakeLiteralName "HasSeenPlayer?") true)
  (bind _enemyisdead (CallFunction|DecreaseHealth Damage))
  (if _enemyisdead
    ;[1 1 1] Attack Player Normally
    (CallFunction|Die)
    (else
      (Animation|Montage|PlayMontage (Variables|Character|GetMesh) "/Game/AI/Weak_Zombie/Animation/Combat/Zombie_Reaction_Hit__1__Montage.Zombie_Reaction_Hit__1__Montage"))))

(event EventBeginPlay
  ;[1 1 1] Setting Enemy Health
  (bind _output_get (Variables|Default|SetEnemyCurrentHealth (Variables|Default|GetEnemyCurrentHealth)))
  (AI|Components|Blackboard|SetValueasFloat (AI|GetBlackboard (AI|GetAIController self)) (Utilities|Name|MakeLiteralName "EnemyHealth") _output_get))

(event EventTick
  (params (DeltaSeconds :type Float%20%28single-precision%29))
  ;[1 1 1] Passive Sound
  (Utilities|FlowControl|Delay 5.0)
  (Audio|PlaySoundatLocation (Utilities|Select :Index (Math|Random|RandomIntegerinRange 0 1) :Option%200 "/Game/Audio/ZombieGroans/ZombieGroan1.ZombieGroan1" :Option%201 "/Game/Audio/ZombieGroans/ZombieGraon2.ZombieGraon2") (Transformation|GetWorldLocation (Variables|Character|GetMesh)) "0, 0, 0" 1.0 1.0 0.0 0 0 0 0))

(fn ConstructionScript)

(fn HitDetection(Left)
  (if (not (Variables|Default|GetHitPlayer))
    (bind _outactors (Actor|GetAllActorsOfClass "/Game/AI/Weak_Zombie/WeakZombie_BP.WeakZombie_BP_C"))
    (bind (_outhit _returnvalue) (Collision|SphereTraceForObjects (Transformation|GetSocketLocation (Variables|Character|GetMesh) "LeftHand") (Transformation|GetSocketLocation (Variables|Character|GetMesh) "LeftHandMiddle3") 5e+01 (Utilities|Array|MakeArray "ObjectTypeQuery3") false _outactors "None"))
    (if _returnvalue
      (bind _asbp_third_person_character (Utilities|Casting|CastToBP_ThirdPersonCharacter (.HitActor (Collision|BreakHitResult _outhit))))
      (if (Variables|/Game/ThirdPerson/Blueprints/BP_ThirdPersonCharacter.BP_ThirdPersonCharacter_C|GetBlocking? _asbp_third_person_character)
        (bind _staminadepleated (Default|DecreaseStamina _asbp_third_person_character 1e+01))
        (if _staminadepleated
          (Default|BrokenGaurd _asbp_third_person_character)
          (else
            (Default|BlockedHit _asbp_third_person_character)
            (Audio|PlaySoundatLocation "/Game/Audio/MainCharacter_SFX/BlockSoundFX.BlockSoundFX" (Transformation|GetWorldLocation (Variables|/Script/Engine.Character|GetMesh _asbp_third_person_character)) "0, 0, 0" 1.0 1.0 0.0 0 0 0 0)))
        (Variables|Default|SetHitPlayer true)
        (else
          (Game|Damage|ApplyDamage _asbp_third_person_character 1e+01 0 0)
          (Variables|Default|SetHitPlayer true))))))

(fn HitDetection(Right)
  (if (not (Variables|Default|GetHitPlayer))
    (bind _outactors (Actor|GetAllActorsOfClass "/Game/AI/Weak_Zombie/WeakZombie_BP.WeakZombie_BP_C"))
    (bind (_outhit _returnvalue) (Collision|SphereTraceForObjects (Transformation|GetSocketLocation (Variables|Character|GetMesh) "RightHand") (Transformation|GetSocketLocation (Variables|Character|GetMesh) "RightHandMiddle3") 5e+01 (Utilities|Array|MakeArray "ObjectTypeQuery3") false _outactors "None"))
    (if _returnvalue
      (bind _asbp_third_person_character (Utilities|Casting|CastToBP_ThirdPersonCharacter (.HitActor (Collision|BreakHitResult _outhit))))
      (if (Variables|/Game/ThirdPerson/Blueprints/BP_ThirdPersonCharacter.BP_ThirdPersonCharacter_C|GetBlocking? _asbp_third_person_character)
        (bind _staminadepleated (Default|DecreaseStamina _asbp_third_person_character 1e+01))
        (if _staminadepleated
          (Default|BrokenGaurd _asbp_third_person_character)
          (Variables|Default|SetHitPlayer true)
          (else
            (Default|BlockedHit _asbp_third_person_character)
            (Audio|PlaySoundatLocation "/Game/Audio/MainCharacter_SFX/BlockSoundFX.BlockSoundFX" (Transformation|GetWorldLocation (Variables|/Script/Engine.Character|GetMesh _asbp_third_person_character)) "0, 0, 0" 1.0 1.0 0.0 0 0 0 0)))
        (else
          (Game|Damage|ApplyDamage _asbp_third_person_character 1e+01 0 0)
          (Variables|Default|SetHitPlayer true))))))

(fn DecreaseHealth
  (params (Damage :type Float%20%28double-precision%29))
  (if (> (Variables|Default|GetEnemyCurrentHealth) 0.0)
    (Variables|Default|SetEnemyCurrentHealth (- (Variables|Default|GetEnemyCurrentHealth) Damage))
    (if (<= (Variables|Default|GetEnemyCurrentHealth) 0.0)
      (return true)
      (else
        (return false)))))